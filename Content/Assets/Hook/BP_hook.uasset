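; Crane hook actor that descends to the finish zone, grabs a character found there and decides the winner of the match.
; TriggerCraneAnime lowers and raises the hook through two Z-position timelines, querying the BP_Finish child actor between them.
; A grabbed character follows AttachPoint every Tick, gets flagged Winning while others get Loosing, and the game mode disables input.
; After the rise and a short delay, the game mode ends the game.
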(event Custom|TriggerCraneAnime
  (if (not (Variables|Default|GetGrabbing))
    (Variables|Default|SetGrabbing true)
    (Audio|PlaySound2D "/Game/Sons/SFX_HookStart.SFX_HookStart" 1.0 1.0 0.0 0 0)
    (bind _crane_position (Timeline|Crane%20Movement PlayFromStart)
      (:Update
        (CallFunction|UpdateCranePosition _crane_position))
      (:Finished
        ;[1 1 1] Try to find a character to grab and grab him
        (bind _asbp_finish (Utilities|Casting|CastToBP_Finish (Variables|/Script/Engine.ChildActorComponent|GetChildActor (Variables|Default|GetFinishZone))))
        (bind (_foundcharacter _characterfound) (Default|TrytoFindCharacter _asbp_finish))
        (Utilities|FlowControl|Sequence
          (:then_0
            (if _foundcharacter
              (CallFunction|GrabCharacter _characterfound)
              (Audio|PlaySound2D "/Game/Sons/SFX_HookClose.SFX_HookClose" 1.0 1.0 0.0 0 0)))
          (:then_1
            (CallFunction|OnTriggerCraneGoingUp)))))))

(event Custom|OnTriggerCraneGoingUp
  (bind _sm_hook_hook3 (Variables|Default|GetSM_Hook_hook3))
  (Utilities|IsValid (Variables|Default|GetGrabbedCharacter)
    (:Is%20Valid
      (bind _outactors (Actor|GetAllActorsOfClass "/Game/SideScrollerCPP/Blueprints/SideScrollerCharacter.SideScrollerCharacter_C"))
      (for _array_element _outactors
        (if (== _array_element (Variables|Default|GetGrabbedCharacter))
          (Variables|/Game/SideScrollerCPP/Blueprints/SideScrollerCharacter.SideScrollerCharacter_C|SetWinning _array_element true)
          (else
            (Variables|/Game/SideScrollerCPP/Blueprints/SideScrollerCharacter.SideScrollerCharacter_C|SetLoosing _array_element true))))
      (bind _asbp_bread_basket_game_mode (Utilities|Casting|CastToBP_BreadBasketGameMode (Game|GetGameMode)))
      (Default|DisableCtrlInput _asbp_bread_basket_game_mode)
      (bind _crane_position (Timeline|Timeline_0 PlayFromStart)
        (:Update
          (CallFunction|UpdateCranePosition _crane_position))
        (:Finished
          (Components|Animation|SetPosition _sm_hook_hook3 0.0 true)
          (Audio|Components|Audio|Stop _sm_hook_hook3)
          (Variables|Default|SetGrabbing false)
          (Utilities|IsValid (Variables|Default|GetGrabbedCharacter)
            (:Is%20Valid
              (Utilities|FlowControl|Delay 3.0)
              (Variables|Default|SetGrabbedCharacter 0)
              (bind _asbp_bread_basket_game_mode_2 (Utilities|Casting|CastToBP_BreadBasketGameMode (Game|GetGameMode)))
              (Default|TriggerGameEnd _asbp_bread_basket_game_mode_2))))))
    (:Is%20Not%20Valid
      (Timeline|Timeline_0 PlayFromStart))))

(event EventBeginPlay)

(event Collision|EventActorBeginOverlap
  (params (OtherActor :type Actor%20Object%20Reference)))

(event EventTick
  (params (DeltaSeconds :type Float%20%28single-precision%29))
  (bind _attachpoint (Variables|Default|GetAttachPoint))
  (bind _grabbedcharacter (Variables|Default|GetGrabbedCharacter))
  (Utilities|IsValid _grabbedcharacter
    (:Is%20Valid
      (Transformation|SetActorLocationAndRotation _grabbedcharacter (Transformation|GetWorldLocation _attachpoint) (Transformation|GetWorldRotation _attachpoint)))))

(fn ConstructionScript)

(fn GrabCharacter
  (params (GrabbedCharacter :type Side%20Scroller%20Character%20Object%20Reference))
  (Audio|Components|Audio|Play (Variables|Default|GetSM_Hook_hook3) false)
  (CallFunction|DisableAllPlayers)
  (Variables|Default|SetGrabbedCharacter GrabbedCharacter))

(fn UpdateCranePosition
  (params (Z :type Float%20%28single-precision%29))
  (bind _returnvalue (Transformation|GetActorLocation))
  (bind (_x _y) (Math|Vector|BreakVector _returnvalue))
  (Transformation|SetActorLocation (Math|Vector|MakeVector _x _y Z) false false))

(fn DisableAllPlayers)