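; Shared game camera that frames two to four players and becomes the view target for every player controller.
; After a brief startup delay it caches the game mode's players, then a fast looping timer runs an update for the player count.
; Each update sets spring arm length to the clamped largest pairwise player distance and interpolates the actor toward their average position.
; An aspect-ratio-scaled distance helper exists but is unused.
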(event Custom|UpdateCamera
  (switch int (Utilities|Array|Length (Variables|Default|GetPlayersReference))
    (:2
      (CallFunction|SetArmLengthP2)
      (CallFunction|SetCamPosP2))
    (:3
      (CallFunction|SetArmLengthP3)
      (CallFunction|SetCamPosP3))
    (:4
      (CallFunction|SetArmLengthP4)
      (CallFunction|SetCamPosP4))))

(event EventBeginPlay
  (Utilities|FlowControl|Delay 0.01)
  (CallFunction|ClassSetup)
  (Utilities|Time|SetTimerbyFunctionName 0 "UpdateCamera" 0.001 true))

(fn ConstructionScript)

(fn ClassSetup
  (bind _asbp_bread_basket_game_mode (Utilities|Casting|CastToBP_BreadBasketGameMode (Game|GetGameMode)))
  (bind _output_get (Variables|Default|SetBP%20Game%20Mode _asbp_bread_basket_game_mode))
  (Variables|Default|SetPlayersReference (Variables|/Game/Blueprints/BP_BreadBasketGameMode.BP_BreadBasketGameMode_C|GetPlayers _output_get))
  (bind _outactors (Actor|GetAllActorsOfClass "/Script/Engine.PlayerController"))
  (Game|Player|SetViewTargetwithBlend _outactors self 0.0 "VTBlend_Linear" 0.0 false)
  (for (_array_element _array_index) (Variables|Default|GetPlayersReference)
    (switch int _array_index
      (:0
        (Variables|Default|SetP1 _array_element))
      (:1
        (Variables|Default|SetP2 _array_element))
      (:2
        (Variables|Default|SetP3 _array_element))
      (:3
        (Variables|Default|SetP4 _array_element)))))

(fn SetArmLengthP4
  (bind _p1 (Variables|Default|GetP1))
  (bind _p2 (Variables|Default|GetP2))
  (bind _p3 (Variables|Default|GetP3))
  (bind _p4 (Variables|Default|GetP4))
  (Variables|/Script/Engine.SpringArmComponent|SetTargetArmLength (Variables|Default|GetSpringArm) (Math|Float|Clamp(Float) (.MaxValue (Math|Float|MaxOfFloatArray (Utilities|Array|MakeArray (Transformation|GetDistanceTo _p1 _p2) (Transformation|GetDistanceTo _p1 _p3) (Transformation|GetDistanceTo _p1 _p4) (Transformation|GetDistanceTo _p2 _p3) (Transformation|GetDistanceTo _p2 _p4) (Transformation|GetDistanceTo _p3 _p4)))) (Variables|Default|GetMinArmLength) (Variables|Default|GetMaxArmLength))))

(fn SetArmLengthP3
  (bind _p1 (Variables|Default|GetP1))
  (bind _p2 (Variables|Default|GetP2))
  (bind _p3 (Variables|Default|GetP3))
  (Variables|/Script/Engine.SpringArmComponent|SetTargetArmLength (Variables|Default|GetSpringArm) (Math|Float|Clamp(Float) (.MaxValue (Math|Float|MaxOfFloatArray (Utilities|Array|MakeArray (Transformation|GetDistanceTo _p1 _p2) (Transformation|GetDistanceTo _p1 _p3) (Transformation|GetDistanceTo _p2 _p3)))) (Variables|Default|GetMinArmLength) (Variables|Default|GetMaxArmLength))))

(fn SetArmLengthP2
  (Variables|/Script/Engine.SpringArmComponent|SetTargetArmLength (Variables|Default|GetSpringArm) (Math|Float|Clamp(Float) (Transformation|GetDistanceTo (Variables|Default|GetP1) (Variables|Default|GetP2)) (Variables|Default|GetMinArmLength) (Variables|Default|GetMaxArmLength))))

(fn SetCamPosP4
  (Variables|Default|SetCurPos (/ (+ (Transformation|GetActorLocation (Variables|Default|GetP1)) (Transformation|GetActorLocation (Variables|Default|GetP2)) (Transformation|GetActorLocation (Variables|Default|GetP3)) (Transformation|GetActorLocation (Variables|Default|GetP4))) (Math|Conversions|ToFloat(Integer) (Utilities|Array|Length (Variables|Default|GetPlayersReference)))))
  (Transformation|SetActorLocation (Math|Interpolation|VInterpTo (Variables|Default|GetPreviousPos) (Variables|Default|GetCurPos) (Utilities|Time|GetWorldDeltaSeconds) (Variables|Default|GetInterpSpeed)) false false)
  (Variables|Default|SetPreviousPos (Transformation|GetActorLocation)))

(fn SetCamPosP3
  (Variables|Default|SetCurPos (/ (+ (Transformation|GetActorLocation (Variables|Default|GetP1)) (Transformation|GetActorLocation (Variables|Default|GetP2)) (Transformation|GetActorLocation (Variables|Default|GetP3))) (Math|Conversions|ToFloat(Integer) (Utilities|Array|Length (Variables|Default|GetPlayersReference)))))
  (Transformation|SetActorLocation (Math|Interpolation|VInterpTo (Variables|Default|GetPreviousPos) (Variables|Default|GetCurPos) (Utilities|Time|GetWorldDeltaSeconds) (Variables|Default|GetInterpSpeed)) false false)
  (Variables|Default|SetPreviousPos (Transformation|GetActorLocation)))

(fn SetCamPosP2
  (Variables|Default|SetCurPos (/ (+ (Transformation|GetActorLocation (Variables|Default|GetP1)) (Transformation|GetActorLocation (Variables|Default|GetP2))) (Math|Conversions|ToFloat(Integer) (Utilities|Array|Length (Variables|Default|GetPlayersReference)))))
  (Transformation|SetActorLocation (Math|Interpolation|VInterpTo (Variables|Default|GetPreviousPos) (Variables|Default|GetCurPos) (Utilities|Time|GetWorldDeltaSeconds) (Variables|Default|GetInterpSpeed)) false false)
  (Variables|Default|SetPreviousPos (Transformation|GetActorLocation)))

(fn GetScaledDistance
  (params (Actor1 :type Actor%20Object%20Reference) (Actor2 :type Actor%20Object%20Reference))
  (bind _returnvalue (Transformation|GetActorLocation Actor2))
  (bind _returnvalue_2 (Game|GetPlayerController 0))
  (bind _returnvalue_3 (Transformation|GetActorLocation Actor1))
  (bind (_sizex _sizey) (HUD|GetViewportSize _returnvalue_2))
  (bind (_x _y _z) (Math|Vector|BreakVector _returnvalue_3))
  (bind (_x_2 _y_2 _z_2) (Math|Vector|BreakVector _returnvalue))
  (Variables|Default|SetAspectRatio (/ (Math|Conversions|ToFloat(Integer) _sizex) (Math|Conversions|ToFloat(Integer) _sizey)))
  (return (Math|Float|Sqrt (* (Math|Float|Square (- _y _y_2)) (Math|Float|Square (* (- _z _z_2) (Variables|Default|GetAspectRatio)))))))