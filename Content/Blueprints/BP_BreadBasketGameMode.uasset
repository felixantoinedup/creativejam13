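; Game mode for BreadBasket that sets up local multiplayer side-scroller matches and runs a start countdown.
; On BeginPlay it creates players up to a maximum count, spawning and possessing a character at each PlayerStart tagged with that player's index.
; Input on the stored characters stays disabled until the printed countdown finishes.
; A GameEnd macro, not called here, disables input, waits briefly and reloads the current level.
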(event EventBeginPlay
  (CallFunction|GetPlayerStartPoints)
  (CallFunction|SpawnPlayers)
  (CallFunction|DisableCtrlInput)
  (Utilities|GameStartCountdown)
  (CallFunction|EnableCtrlInput))

(fn ConstructionScript)

(fn GetPlayerStartPoints
  (bind _outactors (Actor|GetAllActorsOfClass "/Script/Engine.PlayerStart"))
  (Variables|Default|SetPlayerStartArray _outactors))

(fn SpawnPlayers
  (for _index (range 0 (- (Variables|Default|GetMaxPlayerCount) 1))
    (Variables|Default|Setindex _index)
    (for _array_element (Variables|Default|GetPlayerStartArray)
      (if (Utilities|Name|Equal(Name) (Variables|/Script/Engine.PlayerStart|GetPlayerStartTag _array_element) (Utilities|String|StringToName (Utilities|String|ToString(Integer) (Variables|Default|Getindex))))
        (Class|GameplayStatics|CreatePlayer (Variables|Default|Getindex))
        (bind _returnvalue (Game|SpawnActorfromClass "/Game/SideScrollerCPP/Blueprints/SideScrollerCharacter.SideScrollerCharacter_C" (Transformation|GetActorTransform _array_element) "AlwaysSpawn" 0 0))
        (Pawn|Possess (Game|GetPlayerController (Variables|Default|Getindex)) _returnvalue)
        (Utilities|Array|AddUnique (Variables|Default|GetPlayers) _returnvalue)
        (Utilities|Array|AddUnique (Variables|Default|GetPlayerControllers) (Game|GetPlayerController (Variables|Default|Getindex)))))))

(fn DisableCtrlInput
  ;[1 1 1] Disable input for countdown
  (for _index (range 0 (- (Utilities|Array|Length (Variables|Default|GetPlayers)) 1))
    (Input|DisableInput (Utilities|Array|Get(acopy) (Variables|Default|GetPlayers) _index) (Utilities|Array|Get(acopy) (Variables|Default|GetPlayerControllers) _index))))

(fn EnableCtrlInput
  ;[1 1 1] Enable input after countdown
  (for _index (range 0 (- (Utilities|Array|Length (Variables|Default|GetPlayers)) 1))
    (Input|EnableInput (Utilities|Array|Get(acopy) (Variables|Default|GetPlayers) _index) (Utilities|Array|Get(acopy) (Variables|Default|GetPlayerControllers) _index))))