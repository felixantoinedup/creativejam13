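; BP_Finish is a finish trigger for side-scroller characters, but its box overlap event is empty.
; An unwired sequence disables every character's movement, waits briefly, resets positions, then re-enables movement.
; The reset matches each character's array index to a PlayerStart tag and teleports it there.
; An unused helper casts the box's first overlapping actor to a SideScrollerCharacter.
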(event OnComponentBeginOverlap(Box)
  (params (OverlappedComponent :type Primitive%20Component%20Object%20Reference) (OtherActor :type Actor%20Object%20Reference) (OtherComp :type Primitive%20Component%20Object%20Reference) (OtherBodyIndex :type Integer) (bFromSweep :type Boolean) (SweepResult :type Hit%20Result%20Structure%20%28by%20ref%29)))

(fn ConstructionScript)

(fn DisableCtrlInput
  (bind _outactors (Actor|GetAllActorsOfClass "/Game/SideScrollerCPP/Blueprints/SideScrollerCharacter.SideScrollerCharacter_C"))
  (for _index (range 0 (- (Utilities|Array|Length _outactors) 1))
    (Components|Activation|Deactivate (Variables|/Script/Engine.Character|GetCharacterMovement (Utilities|Array|Get(acopy) _outactors _index)))))

(fn ResetPlayerLocation
  (bind _outactors (Actor|GetAllActorsOfClass "/Game/SideScrollerCPP/Blueprints/SideScrollerCharacter.SideScrollerCharacter_C"))
  (for _index (range 0 (- (Utilities|Array|Length _outactors) 1))
    (bind _outactors_2 (Actor|GetAllActorsOfClass "/Script/Engine.PlayerStart"))
    (bind _array_element (Utilities|Array|ForEachLoopwithBreak _outactors_2 :!label _label)
      (:LoopBody
        (if (Utilities|Enum|Equal(Enum) (Utilities|String|ToString(Integer) _index) (Utilities|String|ToString(Name) (Variables|/Script/Engine.PlayerStart|GetPlayerStartTag _array_element)))
          (goto _label Break)))
      (:Completed
        (Transformation|SetActorRelativeLocation (Utilities|Array|Get(acopy) _outactors _index) (Transformation|GetActorLocation _array_element) false true)))))

(fn EnableCtrlInput
  (bind _outactors (Actor|GetAllActorsOfClass "/Game/SideScrollerCPP/Blueprints/SideScrollerCharacter.SideScrollerCharacter_C"))
  (for _index (range 0 (- (Utilities|Array|Length _outactors) 1))
    (Components|Activation|Activate (Variables|/Script/Engine.Character|GetCharacterMovement (Utilities|Array|Get(acopy) _outactors _index)) false)))

(fn TrytoFindCharacter
  (bind _box (Variables|Default|GetBox))
  (bind _overlappingactors (Collision|GetOverlappingActors _box 0 :!class /Script/Engine.PrimitiveComponent))
  (if (> (Utilities|Array|Length _overlappingactors) 0)
    (bind _asside_scroller_character (Utilities|Casting|CastToSideScrollerCharacter (Utilities|Array|Get(acopy) _overlappingactors)))
    (return true _asside_scroller_character)
    (else
      (return false 0))))